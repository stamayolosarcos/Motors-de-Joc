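; Cinematic controller actor that plays a level sequence when the game begins, locking out player input for its duration.
; BeginPlay creates and plays a sequence player, disables the player pawn's input and removes all widgets.
; Tick compares playback time to the end time; once reached, it creates the HUD behind a validity check, adds it to the viewport and re-enables input, with no guard against repeating each frame.
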(event EventBeginPlay
  (bind (_outactor _returnvalue) (Sequencer|Player|CreateLevelSequencePlayer (Variables|Default|GetLevelSequence)))
  (Sequencer|Player|Play _returnvalue :!class /Script/MovieScene.MovieSceneSequencePlayer)
  (Input|DisableInput (Game|Player|GetPlayerPawn 0) (Game|GetPlayerController 0))
  (Viewport|RemoveAllWidgets))

(event Collision|EventActorBeginOverlap
  (params (OtherActor :type Actor%20Object%20Reference)))

(event EventTick
  (params (DeltaSeconds :type Float%20%28single-precision%29))
  (if (>= (Class|TimeManagementBlueprintLibrary|ToSeconds(QualifiedFrameTime) (Sequencer|Player|GetCurrentTime (Variables|/Script/LevelSequence.LevelSequenceActor|GetSequencePlayer (stale EventBeginPlay _outactor)))) (Class|TimeManagementBlueprintLibrary|ToSeconds(QualifiedFrameTime) (Class|MovieSceneSequencePlayer|GetEndTime (Variables|/Script/LevelSequence.LevelSequenceActor|GetSequencePlayer (stale EventBeginPlay _outactor)))))
    (Utilities|FlowControl|Sequence
      (:then_0
        (Utilities|IsValid 0
          (:Is%20Valid
            _)
          (:Is%20Not%20Valid
            (bind _returnvalue (UserInterface|CreateWidget "/Game/HUD/HUD.HUD_C" (Game|GetPlayerController 0)))
            (Variables|Default|SetHUD _returnvalue)))
        (UserInterface|Viewport|AddtoViewport (Variables|Default|GetHUD) 0))
      (:then_1
        (Input|EnableInput (Game|Player|GetPlayerPawn 0) (Game|GetPlayerController 0))))))

(fn ConstructionScript)